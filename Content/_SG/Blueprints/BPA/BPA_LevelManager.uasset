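; BPA_LevelManager is a level manager actor that provides pooled bullets, registering itself on the game instance at BeginPlay.
; PoolingBullets reuses the first bullet in an available state, or spawns a new BPA_Bullet away at a fixed location and adds it to the pool.
; It then configures that bullet's scale, damage, velocity, target tag, causer, flipbook and lifespan before moving it to the requested location.
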(event `self.ReceiveBeginPlay`
  (set `/Game/_SG/Data/GI_Game.Ref_LevelManager` self (`/Game/_SG/Data/BFL_Game.BFL_GetGI`)))

(event `self.ReceiveTick`
  (params (DeltaSeconds :type "Float (single-precision)"))
  ;[0 0 0] 调试池子里有多少个对象
)

(fn `PoolingBullets`
  (params (Location :type "Vector Structure") (Scale :type "Vector Structure") (Damage :type "Float (double-precision)") (ProjectileVelocity :type "Vector Structure") (TargetTag :type Name) (DamageCauser :type "Actor Object Reference") (Flipbook :type "PaperFlipbook Object Reference") (FlipbookScale :type "Vector Structure") (LifeSpan :type "Float (double-precision)"))
  (locals (AvailableBullet :type "/Game/_SG/Blueprints/BPA/BPA_Bullet Object Reference"))
  (bind _availablebullet (`local.AvailableBullet`))
  (for _array_element (`self.BulletPool`)
    (if (`|EnumEquality` (`/Game/_SG/Blueprints/BPA/BPA_Bullet.BulletState` _array_element) "NewEnumerator1")
      (set `local.AvailableBullet` _array_element)
      (break)))
  (`local.AvailableBullet`
    (:`then`
      _)
    (:`else`
      (bind _returnvalue (`|SpawnActorFromClass` "/Game/_SG/Blueprints/BPA/BPA_Bullet.BPA_Bullet_C" (`KismetMathLibrary.MakeTransform` (1000.0 1000.0 -1000.0)) "AdjustIfPossibleButAlwaysSpawn" "MultiplyWithRoot" null "None" (0.0 0.0 0.0) null))
      (bind _output_get (set `local.AvailableBullet` _returnvalue))
      (`KismetArrayLibrary.Array_Add` (`self.BulletPool`) _output_get)))
  (`/Game/_SG/Blueprints/BPA/BPA_Bullet.SetupBulletProp` _availablebullet (`local.Scale`) (`local.Damage`) (`local.ProjectileVelocity`) (`local.TargetTag`) (`local.DamageCauser`) (`local.Flipbook`) (`local.FlipbookScale`) (`local.LifeSpan`))
  (`self.K2_SetActorLocation` _availablebullet (`local.Location`) false false))

(fn `UserConstructionScript`)