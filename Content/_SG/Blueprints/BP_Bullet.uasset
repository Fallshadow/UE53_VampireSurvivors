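; BP_Bullet is a projectile that detects hits on actors carrying a target tag; no damage is applied here.
; On BeginPlay it sets its projectile movement velocity from ProjectileVelocity.
; Sphere overlaps with new tagged actors record the hit in a no-repeat list, print the name and destroy the bullet after a brief delay.
; Other valid overlaps trigger a longer, temporary delayed destroy.
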(event `self.ReceiveBeginPlay`
  (set `MovementComponent.Velocity` (`self.ProjectileVelocity`) (`self.ProjectileMovement`)))

(event `self.Sphere.OnComponentBeginOverlap`
  (params (OverlappedComponent :type "PrimitiveComponent Object Reference") (OtherActor :type "Actor Object Reference") (OtherComp :type "PrimitiveComponent Object Reference") (OtherBodyIndex :type Integer) (bFromSweep :type Boolean) (SweepResult :type "HitResult Structure (by ref)"))
  (`/Engine/EditorBlueprintResources/StandardMacros.IsValid` OtherActor
    (:`Is Valid`
      (if (and (`self.ActorHasTag` OtherActor (`self.TargetTag`)) (not (`KismetArrayLibrary.Array_Contains` (`self.DamagedActorList`) OtherActor)))
        (bind _output_get (set `self.HitTarget` OtherActor))
        (`KismetArrayLibrary.Array_AddUnique` (`self.DamagedActorList`) _output_get)
        (`KismetSystemLibrary.PrintString` (`KismetSystemLibrary.GetDisplayName` (`self.HitTarget`)) true true (struct :`R` 1.0 :`G` 1.0 :`B` 1.0 :`A` 1.0))
        (`KismetSystemLibrary.Delay` 0.05)
        (`self.K2_DestroyActor`)
        (else
          ;[0.2712 1 0.2329] Temp
          (`KismetSystemLibrary.Delay` 2.0)
          (`self.K2_DestroyActor`))))))

(fn `UserConstructionScript`)