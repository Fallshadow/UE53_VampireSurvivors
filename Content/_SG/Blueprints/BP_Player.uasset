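; BP_Player is the player-controlled Blueprint that handles movement input.
; On BeginPlay it casts its controller to PC_InGame and adds the IMC_SG Enhanced Input mapping context.
; IA_Movement feeds movement input along world X and Y axes rather than control rotation, gated by a GeneralCheck macro that tests whether the player is not dead.
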(event `self.ReceiveBeginPlay`
  (bind _aspc_in_game (cast `/Game/_SG/Data/PC_InGame` (`self.GetController`)))
  (bind _returnvalue (pcsubsystem `EnhancedInputLocalPlayerSubsystem` _aspc_in_game))
  (`/Engine/EditorBlueprintResources/StandardMacros.IsValid` _returnvalue
    (:`Is Valid`
      (`EnhancedInputSubsystemInterface.AddMappingContext` _returnvalue "/Game/_SG/Inputs/IMC_SG.IMC_SG" 0 (struct)))))

(event `EnhancedInput|/Game/_SG/Inputs/IA_Movement`
  (params (ActionValue :type "Vector2D Structure") (ElapsedSeconds :type "Float (double-precision)") (TriggeredSeconds :type "Float (double-precision)") (InputAction :type "InputAction Object Reference" :default "/Game/_SG/Inputs/IA_Movement.IA_Movement"))
  (bind (_x _y) (`KismetMathLibrary.BreakVector2D` ActionValue))
  (:`Triggered`
    (`self.GeneralCheck`
      (:`true`
        (set `self.ActionValX` _x)
        (set `self.ActionValY` _y)
        (`self.AddMovementInput` (1.0 0.0 0.0) (`self.ActionValX`))
        (`self.AddMovementInput` (0.0 1.0 0.0) (`self.ActionValY`))))))

(fn `UserConstructionScript`)